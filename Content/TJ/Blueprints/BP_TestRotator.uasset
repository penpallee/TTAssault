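; BP_TestRotator is a test actor that uses a RotatingMovement component with a pivot taken from the player character's position.
; On Tick, a DoOnce gate sets the pivot translation to the world-space offset from the actor to the player's BP_ThirdPersonCharacter and prints it.
; A six-second Delay then resets the gate, so the pivot refreshes periodically instead of every frame.
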(event EventBeginPlay)

(event Collision|EventActorBeginOverlap
  (params (OtherActor :type Actor%20Object%20Reference)))

(event EventTick
  (params (DeltaSeconds :type Float%20%28single-precision%29))
  (Utilities|FlowControl|DoOnce false :!label _label
    (:Completed
      (bind _asbp_third_person_character (Utilities|Casting|CastToBP_ThirdPersonCharacter (Game|GetPlayerCharacter 0)))
      (bind _output_get (Variables|/Script/Engine.RotatingMovementComponent|SetPivotTranslation (Variables|Default|GetRotatingMovement) (- (Transformation|GetActorLocation _asbp_third_person_character) (Transformation|GetActorLocation))))
      (Development|PrintString (Utilities|String|ToString(Vector) _output_get))
      (Utilities|FlowControl|Delay 6.0)
      (goto _label Reset))))

(fn ConstructionScript)