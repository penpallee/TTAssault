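; Assault boss actor that spawns a separate BP_BossHPBar on BeginPlay and keeps it at a fixed vertical offset below itself every Tick.
; Setter functions configure BossMoveComp's speed, homing acceleration and homing target, so the boss moves like a homing projectile.
; GetHPPercentage exposes HP as a fraction of MaxHP.
; SetMode, its OnRep and the collision events are empty stubs, with the visibility-switch logic left disconnected.
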(event OnComponentHit(CapsuleComponent)
  (params (HitComponent :type Primitive%20Component%20Object%20Reference) (OtherActor :type Actor%20Object%20Reference) (OtherComp :type Primitive%20Component%20Object%20Reference) (NormalImpulse :type Vector :default "0, 0, 0") (Hit :type Hit%20Result%20Structure%20%28by%20ref%29)))

(event OnComponentBeginOverlap(CapsuleComponent)
  (params (OverlappedComponent :type Primitive%20Component%20Object%20Reference) (OtherActor :type Actor%20Object%20Reference) (OtherComp :type Primitive%20Component%20Object%20Reference) (OtherBodyIndex :type Integer) (bFromSweep :type Boolean) (SweepResult :type Hit%20Result%20Structure%20%28by%20ref%29)))

(event EventBeginPlay
  (bind _returnvalue (Game|SpawnActorfromClass "/Game/TJ/Blueprints/BP_BossHPBar.BP_BossHPBar_C" (Math|Transform|MakeTransform (Transformation|GetActorLocation) "0, 0, 0" "1.000000,1.000000,1.000000") "Undefined" 0 0)))

(event EventTick
  (params (DeltaSeconds :type Float%20%28single-precision%29))
  (bind _returnvalue (Transformation|GetActorLocation))
  (Transformation|SetActorLocation (stale EventBeginPlay _returnvalue) (Math|Vector|MakeVector (.x _returnvalue) (.y _returnvalue) (- (.z _returnvalue) 1.8e+02)) false false))

(event Collision|EventActorBeginOverlap
  (params (OtherActor :type Actor%20Object%20Reference)))

(event Input|ActionEvents|InputActionDash
  (params (Key :type Key%20Structure :default "None")))

(event Input|ActionEvents|InputActionTestPushAttack
  (params (Key :type Key%20Structure :default "None")))

(fn ConstructionScript)

(fn SetMode
  (params (mode :type Integer)))

(fn OnRepMode)

(fn SetProjectileSpeed
  (params (InitialSpeed :type Float%20%28double-precision%29) (MaxSpeed :type Float%20%28double-precision%29))
  (bind _bossmovecomp (Variables|Default|GetBossMoveComp))
  (Variables|/Script/Engine.ProjectileMovementComponent|SetMaxSpeed _bossmovecomp MaxSpeed)
  (Variables|/Script/Engine.ProjectileMovementComponent|SetInitialSpeed _bossmovecomp InitialSpeed))

(fn SeProjectileHomingAccelerationMagnitude
  (params (Magnitude :type Float%20%28double-precision%29))
  (Variables|/Script/Engine.ProjectileMovementComponent|SetHomingAccelerationMagnitude (Variables|Default|GetBossMoveComp) Magnitude))

(fn SetHomingTargetComponent
  (params (TargetComponent :type Scene%20Component%20Object%20Reference))
  (Variables|/Script/Engine.ProjectileMovementComponent|SetHomingTargetComponent (Variables|Default|GetBossMoveComp) TargetComponent))

(fn GetHPPercentage
  (return (/ (Variables|Default|GetHP) (Variables|Default|GetMaxHP))))