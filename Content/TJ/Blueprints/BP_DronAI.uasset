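; Drone AI actor whose spinning sphere roams between five arrow-marked points, picking a random one every 1 to 3 seconds.
; A self-restarting timer lerps the sphere a small fixed fraction toward the target each step, giving an eased glide.
; BeginPlay also repeatedly calls ShootAtPlayer, but that event is empty; the aim-at-player and spawn nodes are disconnected, so it never fires.
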(event Custom|Moving
  (bind _sphere (Variables|Default|GetSphere))
  (Variables|Default|SetAlpha 0.0)
  (Utilities|Time|SetTimerbyEvent (delegate Custom|Moving) 0.02)
  (Variables|Default|SetAlpha (+ (Variables|Default|GetAlpha) 0.04))
  (Transformation|SetWorldLocation _sphere (Math|Vector|Lerp(Vector) (Transformation|GetWorldLocation _sphere) (Variables|Default|GetLocationToMove) (Variables|Default|GetAlpha)) false false))

(event Custom|FindNextDestination
  (bind _arrow1 (Variables|Default|GetArrow1))
  (bind _arrow2 (Variables|Default|GetArrow2))
  (bind _arrow3 (Variables|Default|GetArrow3))
  (bind _arrow4 (Variables|Default|GetArrow4))
  (bind _arrow (Variables|Default|GetArrow))
  (bind _array (Utilities|Array|MakeArray _arrow1 _arrow2 _arrow3 _arrow4 _arrow))
  (Variables|Default|SetLocationToMove (Transformation|GetWorldLocation (Utilities|Array|Get(acopy) _array (Math|Random|RandomIntegerinRange 0 (Utilities|Array|LastIndex _array)))))
  (CallFunction|Moving)
  (Utilities|FlowControl|Delay (Math|Random|RandomFloatinRange 1.0 3.0))
  (CallFunction|FindNextDestination))

(event Custom|ShootAtPlayer)

(event EventBeginPlay
  (CallFunction|FindNextDestination)
  (CallFunction|ShootatPlayer :!label _label)
  (Utilities|FlowControl|Delay 2.0)
  (goto _label))

(event Collision|EventActorBeginOverlap
  (params (OtherActor :type Actor%20Object%20Reference)))

(event EventTick
  (params (DeltaSeconds :type Float%20%28single-precision%29))
  (Transformation|AddLocalRotation (Variables|Default|GetSphere) "0,1.000000, 0" false false))

(fn ConstructionScript)