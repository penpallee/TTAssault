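; BP_Bullet_MultiInductionFire is a timed bullet that bursts into a ring of BP_Bullet_InductionFire projectiles.
; After a short delay from BeginPlay it calls DestroyActor, then spawns twelve enlarged child bullets at its location through a DoOnce.
; Each child's rotation composes a fixed 90-degree offset with an evenly stepped yaw via quaternion multiplication, and the trail sound plays once per spawn.
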(event EventBeginPlay
  (Utilities|FlowControl|Delay 2.0)
  (Actor|DestroyActor)
  (Utilities|FlowControl|DoOnce false
    (:Completed
      (for _index (range 0 11)
        (Game|SpawnActorfromClass "/Game/TJ/Blueprints/BP_Bullet_InductionFire.BP_Bullet_InductionFire_C" (Math|Transform|MakeTransform (Transformation|GetActorLocation) (Class|KismetMathLibrary|QuatRotator (* (Math|Conversions|ToQuaternion(Rotator) "90.000000, 0, 0") (Math|Conversions|ToQuaternion(Rotator) (Math|Rotator|MakeRotator 0.0 0.0 (Math|Conversions|ToFloat(Integer) (* _index 30)))))) "2.000000,2.000000,2.000000") "Undefined" 0 0)
        (Audio|PlaySoundatLocation "/Game/TJ/Resource/Sound_IndectionFireTrail2.Sound_IndectionFireTrail2" (Transformation|GetActorLocation) "0, 0, 0" 1.0 1.0 0.0 0 0 0 0)))))

(event Collision|EventActorBeginOverlap
  (params (OtherActor :type Actor%20Object%20Reference)))

(event EventTick
  (params (DeltaSeconds :type Float%20%28single-precision%29)))

(fn ConstructionScript)