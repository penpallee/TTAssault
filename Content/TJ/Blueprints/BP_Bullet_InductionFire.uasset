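; BP_Bullet_InductionFire is a homing bullet that chases the first player character.
; On BeginPlay it sets the player's capsule as the homing target of its movement component, and every Tick it rotates to face the player's location.
; It also looks up and casts to BP_AssaultBoss without using the result.
; Overlaps only print the other actor's name, with no damage or destroy logic in these graphs.
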(event EventBeginPlay
  (Variables|/Script/Engine.ProjectileMovementComponent|SetHomingTargetComponent (Variables|Default|GetbulletMovementComp) (Variables|/Script/Engine.Character|GetCapsuleComponent (Game|GetPlayerCharacter 0)))
  (bind _returnvalue (Actor|GetActorOfClass "/Game/TJ/Blueprints/BP_AssaultBoss.BP_AssaultBoss_C"))
  (Utilities|Casting|CastToBP_AssaultBoss _returnvalue))

(event Collision|EventActorBeginOverlap
  (params (OtherActor :type Actor%20Object%20Reference))
  (Development|PrintString (Utilities|GetDisplayName OtherActor)))

(event EventTick
  (params (DeltaSeconds :type Float%20%28single-precision%29))
  (Transformation|SetActorRotation (Math|Rotator|FindLookatRotation (Transformation|GetActorLocation) (Transformation|GetActorLocation (Game|GetPlayerCharacter 0)))))

(fn ConstructionScript)