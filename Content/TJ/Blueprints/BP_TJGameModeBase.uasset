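; Game mode that pauses play behind a start widget at launch, drives the minimap markers and ends play when the boss's HP runs out.
; BeginPlay spawns a minimap camera and an assault sign, which Tick moves to the player's and assault boss's Y/Z respectively, each at a fixed X.
; At near-zero BossHP, Tick waits briefly, clears all widgets and pauses.
; A separate event creates a second player as BP_Danmoozi.
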(event Custom|SpawnPlayer2
  (Variables|Default|SetDefaultPawnClass "/Game/TH/Blueprints/BP_Danmoozi.BP_Danmoozi_C")
  (Class|GameplayStatics|CreatePlayer -1))

(event EventBeginPlay
  (bind _returnvalue (Math|Vector|GetForwardVector "0, 0, 0"))
  (Game|SetGamePaused true)
  (bind _returnvalue_2 (UserInterface|CreateWidget "/Game/TJ/UI/WBP_GameStart.WBP_GameStart_C"))
  (UserInterface|Viewport|AddtoViewport _returnvalue_2 0)
  (bind _returnvalue_3 (Game|SpawnActorfromClass "/Game/TJ/Blueprints/BP_MinimapCamera.BP_MinimapCamera_C" (Math|Transform|MakeTransform (Math|Vector|MakeVector -3e+03 (.y _returnvalue) (.z _returnvalue)) (Math|Rotator|FindLookatRotation (Transformation|GetActorLocation) (Transformation|GetActorLocation)) "1.000000,1.000000,1.000000") "Undefined" 0 0))
  (bind _returnvalue_4 (Game|SpawnActorfromClass "/Game/TJ/Blueprints/BP_AssaultSignOnMap.BP_AssaultSignOnMap_C" (Math|Transform|MakeTransform (Math|Vector|MakeVector 0.0 0.0 0.0) "0, 0, 0" "1.000000,1.000000,1.000000") "Undefined" 0 0)))

(event EventTick
  (params (DeltaSeconds :type Float%20%28single-precision%29))
  (bind _returnvalue (Game|GetPlayerCharacter 0))
  (bind _returnvalue_2 (Transformation|GetActorLocation _returnvalue))
  (Utilities|Casting|CastToBP_Danmoozi _returnvalue)
  (bind _returnvalue_3 (Actor|GetActorOfClass "/Game/TJ/Blueprints/BP_AssaultBoss.BP_AssaultBoss_C"))
  (bind _asbp_assault_boss (Utilities|Casting|CastToBP_AssaultBoss _returnvalue_3))
  (Transformation|SetActorLocation (stale EventBeginPlay _returnvalue_3) (Math|Vector|MakeVector -3e+03 (.y _returnvalue_2) (.z _returnvalue_2)) false false)
  (Transformation|SetActorLocation (stale EventBeginPlay _returnvalue_4) (Math|Vector|MakeVector -4.5e+03 (.y (Transformation|GetActorLocation _asbp_assault_boss)) (.z (Transformation|GetActorLocation _asbp_assault_boss))) false false)
  (if (<= (Variables|Default|GetBossHP) 0.1)
    (Utilities|FlowControl|Delay 2.0)
    (Viewport|RemoveAllWidgets)
    (Game|SetGamePaused true)))

(event EventInitializeHUDforPlayer
  (params (NewPlayer :type Player%20Controller%20Object%20Reference)))

(fn ConstructionScript)