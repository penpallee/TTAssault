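; BP_Soondae is a player character that faces the mouse cursor and has a booster-fuelled dash.
; Tick rotates it toward the cursor hit, deriving roll from yaw when pitched upward.
; Dash spends Booster, launches along Direction with sound and Niagara effect, and raises Speed until release; a short Stop timer zeroes velocity and re-arms it.
; GetAngle and IsMouseUpPosition are uncalled helpers, and the authority-based player index branch never runs.
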(event EventBeginPlay
  (Variables|/Script/Engine.PlayerController|SetbShowMouseCursor (Game|GetPlayerController 0) true))

(event EventTick
  (params (DeltaSeconds :type Float%20%28single-precision%29))
  (bind _returnvalue (Game|GetPlayerController 0))
  (bind _returnvalue_2 (Transformation|GetActorLocation))
  (bind _looklayer (Variables|Default|GetLookLayer))
  (bind _hitresult (Class|PlayerController|GetHitResultUnderCursorforObjects _returnvalue _looklayer true))
  (bind _impactpoint (Collision|BreakHitResult _hitresult))
  (bind _returnvalue_3 (Math|Rotator|FindLookatRotation _returnvalue_2 _impactpoint))
  (if (> (.pitch _returnvalue_3) 0.0)
    (Transformation|SetActorRotation (Math|Rotator|MakeRotator (+ -1e+02 (Math|Float|Absolute(Float) (.yaw _returnvalue_3))) (.pitch _returnvalue_3) (.yaw _returnvalue_3)))
    (else
      (Transformation|SetActorRotation (Math|Rotator|MakeRotator (.roll _returnvalue_3) (.pitch _returnvalue_3) (.yaw _returnvalue_3))))))

(event Input|ActionEvents|InputActionDash
  (params (Key :type Key%20Structure :default "None"))
  (bind _returnvalue (Transformation|GetActorRotation))
  (bind _returnvalue_2 (Transformation|GetActorLocation))
  (:Pressed
    (if (and (> (Variables|Default|Getbooster) (Variables|Default|GetboosterLose)) (Variables|Default|GetCool))
      (Audio|PlaySoundatLocation "/Engine/EditorSounds/GamePreview/EjectFromPlayer.EjectFromPlayer" (Transformation|GetActorLocation) "0, 0, 0" 1.0 1.0 0.0 0 0 0 0)
      (Utilities|Time|ClearTimerbyFunctionName 0 "Stop")
      (Character|LaunchCharacter (* (Math|Vector|Normalize (Variables|Default|Getdirection)) 1e+03) false false)
      (if (< (Math|Float|Absolute(Float) (.pitch _returnvalue)) 8.0)
        (Niagara|SpawnSystematLocation "/Game/TH/N_Test.N_Test" _returnvalue_2 (Math|Rotator|MakeRotator (.roll _returnvalue) (+ (.pitch _returnvalue) 16.0) (.yaw _returnvalue)))
        (else
          (Niagara|SpawnSystematLocation "/Game/TH/N_Test.N_Test" _returnvalue_2 (Math|Rotator|MakeRotator (.roll _returnvalue) (.pitch _returnvalue) (.yaw _returnvalue)))))
      (Utilities|Time|SetTimerbyFunctionName 0 "Stop" 0.05)
      (Variables|Default|SetCool false)
      (Variables|Default|Setspeed 1.4e+03)
      (Variables|Default|Setbooster (- (Variables|Default|Getbooster) (Variables|Default|GetboosterLose)))))
  (:Released
    (Variables|Default|Setspeed 1e+03)))

(fn ConstructionScript)

(fn Stop
  (Variables|/Script/Engine.MovementComponent|SetVelocity (Variables|Character|GetCharacterMovement) "0, 0, 0")
  (Variables|Default|SetCool true))

(fn GetAngle
  (params (A :type Vector) (B :type Vector))
  (bind _returnvalue (Math|Vector|Normalize B))
  (bind _returnvalue_2 (Math|Vector|Normalize A))
  (Utilities|FlowControl|Sequence
    (:then_0
      (LocalVariables|SetdegreeAngle (Math|Trig|RadiansToDegrees (Math|Trig|Acos(Degrees) (Math|Vector|DotProduct _returnvalue_2 _returnvalue))))
      (if (< (.z (Math|Vector|CrossProduct _returnvalue_2 _returnvalue)) 0.0)
        (bind _output_get (LocalVariables|SetdegreeAngle (* (LocalVariables|GetdegreeAngle) -1.0))))
      (Development|PrintString (Utilities|String|ToString(Float) _output_get)))
    (:then_1
      (return (LocalVariables|GetdegreeAngle)))))

(fn IsMouseUpPosition
  (params (angle :type Float%20%28double-precision%29))
  (return (Math|Boolean|ORBoolean (> angle 315.0) (< angle 45.0) (and (> angle 135.0) (< angle 225.0)))))