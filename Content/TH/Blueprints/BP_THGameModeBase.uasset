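; Game mode Blueprint that spawns and possesses player characters at the level's PlayerStarts.
; A custom event takes the new player and uses a SwitchHasAuthority to spawn BP_Soondae on Authority or BP_Danmoozi on Remote.
; An incrementing SpawnOrder index picks the PlayerStart for each spawn.
; The event then calls OpenLevel on the localhost address, and nothing in this graph calls the event.
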(event Custom|CustomEvent
  (params (NewPlayer :type Player%20Controller%20Object%20Reference))
  ;[1 1 1] Spawn players at player starts
  (bind _outactors (Actor|GetAllActorsOfClass "/Script/Engine.PlayerStart")) ; Find the player starts in the level
  (Networking|SwitchHasAuthority
    (:Authority
      (bind _returnvalue (Game|SpawnActorfromClass "/Game/TH/Blueprints/BP_Soondae.BP_Soondae_C" (Transformation|GetActorTransform (Utilities|Array|Get(acopy) _outactors (Variables|Default|Getspawn%20order))) "AdjustIfPossibleButDontSpawnIfColliding" 0 0)) ; Spawn a pawn at the specified player start
      (Pawn|Possess NewPlayer _returnvalue))
    (:Remote
      (bind _returnvalue_2 (Game|SpawnActorfromClass "/Game/TH/Blueprints/BP_Danmoozi.BP_Danmoozi_C" (Transformation|GetActorTransform (Utilities|Array|Get(acopy) _outactors (Variables|Default|Getspawn%20order))) "AdjustIfPossibleButDontSpawnIfColliding" 0 0)) ; Spawn a pawn at the specified player start
      (Pawn|Possess NewPlayer _returnvalue_2)))
  (Variables|Default|Setspawn%20order (+ (Variables|Default|Getspawn%20order) 1))
  (Game|OpenLevel(byName) "127.0.0.1"))

(event EventBeginPlay)

(event EventTick
  (params (DeltaSeconds :type Float%20%28single-precision%29)))

(fn ConstructionScript)